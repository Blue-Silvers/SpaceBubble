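; Octopus character that seeks out an assigned bubble and pops it after a delay, notifying its parent BP_Portal.
; Tick drives AI MoveTo, cosine bobbing, a camera-facing health bar and death removal from the portal's list.
; Speeds and timings come from a data asset.
; Classic damage halves walk speed, while a poison effect drains health through repeated gameplay-task delays, though damage handling only records the classic type.
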(event Custom|Pop_Bubble
  (bind _bubbletarget (Variables|Default|GetBubbleTarget))
  ;[0 0.1856 1] Bubble Popped
  (Utilities|FlowControl|Delay (Variables|/Game/Data_Assets/BP_DataAssets/BP_DataAssets_Octopus.BP_DataAssets_Octopus_C|GetBubble_Pop_Time (Variables|Default|GetDataAssets_Octopus)))
  (if (Utilities|Array|ContainsItem (Collision|GetOverlappingActors (Variables|Default|GetSphere) "/Game/GPE/BP_Bubble.BP_Bubble_C" :!class /Script/Engine.PrimitiveComponent) (Variables|Default|GetBubbleTarget))
    (bind _asbp_portal (Utilities|Casting|CastToBP_Portal (Variables|Default|GetParent)))
    (Utilities|Array|RemoveItem (Variables|/Game/GPE/BP_Portal.BP_Portal_C|GetAll_Bubbles _asbp_portal) _bubbletarget)
    (bind _asbp_bubble (Utilities|Casting|CastToBP_Bubble _bubbletarget))
    (Default|Kill _asbp_bubble)
    (Default|BubblePopped _asbp_portal)
    (CallFunction|ResetPopBubble)))

(event Custom|Movement
  ;[1 0.4532 0] Movement
  (if (Utilities|IsValid (Variables|Default|GetBubbleTarget))
    (AI|Navigation|MovetoActor (AI|GetAIController self) (Variables|Default|GetBubbleTarget) 1.5e+02 true true true 0)
    (if (Utilities|IsValid self)
      (if (< (Math|Vector|Distance(Vector) (Transformation|GetActorLocation (Variables|Default|GetBubbleTarget)) (Transformation|GetActorLocation self)) 2e+02)
        (Utilities|FlowControl|DoOnce false
          (:Completed
            (CallFunction|PopBubble))))
      (else
        (Utilities|Platform|CollectGarbage)))))

(event Custom|Check%20Health
  ;[1 0.02291 0] Health System
  (if (< (Variables|Default|GetHealth) 0.0)
    (bind _asbp_portal (Utilities|Casting|CastToBP_Portal (Variables|Default|GetParent)))
    (Utilities|Array|RemoveItem (Variables|/Game/GPE/BP_Portal.BP_Portal_C|GetAll_Ducks _asbp_portal) self)
    (Actor|DestroyActor)))

(event Custom|Buyancy
  (bind _dataassets_octopus (Variables|Default|GetDataAssets_Octopus))
  ;[0 0.6282 1] Buoyancy
  (Transformation|AddActorWorldOffset (Math|Vector|MakeVector 0.0 0.0 (* (Math|Trig|Cos(Radians) (* (Actor|GetGameTimeSinceCreation) (Variables|/Game/Data_Assets/BP_DataAssets/BP_DataAssets_Octopus.BP_DataAssets_Octopus_C|GetDuck_Buoyancy_Speed _dataassets_octopus))) (Variables|/Game/Data_Assets/BP_DataAssets/BP_DataAssets_Octopus.BP_DataAssets_Octopus_C|GetDuck_Buoyancy_Height _dataassets_octopus)))))

(event Custom|Update%20HealthBar
  ;[1 0 0.1599] UI HealthBar
  (if (Utilities|IsValid (Variables|Default|GetHealthBar%20Slider))
    (Transformation|SetWorldRotation (Variables|Default|GetHealthBar) (Math|Rotator|FindLookatRotation (Transformation|GetWorldLocation (Variables|Default|GetHealthBar)) (Transformation|GetWorldLocation (Variables|/Script/Engine.PlayerCameraManager|GetTransformComponent (Game|GetPlayerCameraManager 0)))) false false)
    (Progress|SetPercent (Variables|Default|GetHealthBar%20Slider) (/ (Variables|Default|GetHealth) (Variables|/Game/Data_Assets/BP_DataAssets/BP_DataAssets_Octopus.BP_DataAssets_Octopus_C|GetMax_Health (Variables|Default|GetDataAssets_Octopus))))
    (else
      (Utilities|Platform|CollectGarbage))))

(event Custom|Effects
  ;[0.3596 1 0] Effects
  (if (== (Variables|Default|GetCurrent_Effect) "/Game/GPE/Damage_Type/DT_Poison.DT_Poison")
    (Utilities|FlowControl|DoOnce false
      (:Completed
        (GameplayTasks|TaskWaitDelay (Variables|Default|GetTaskWait) 1.0
          (:then
            (Math|Float|DecrementFloat (Variables|Default|GetHealth)))
          (:OnFinish
            (CallFunction|EffectsReset)))))))

(event Custom|Effects_Reset
  ;[0.3596 1 0] Effects
  (Utilities|FlowControl|DoOnce false) ; enters at Reset
)

(event Custom|Reset_Pop_Bubble
  ;[1 0.4532 0] Movement
  (Utilities|FlowControl|DoOnce false) ; enters at Reset
)

(event EventBeginPlay
  (bind _charactermovement (Variables|Character|GetCharacterMovement))
  (bind _dataassets_octopus (Variables|Default|GetDataAssets_Octopus))
  (Variables|/Script/Engine.CharacterMovementComponent|SetMaxWalkSpeed _charactermovement (Math|Conversions|ToFloat(Integer) (Variables|/Game/Data_Assets/BP_DataAssets/BP_DataAssets_Octopus.BP_DataAssets_Octopus_C|GetSpeed _dataassets_octopus)))
  (Variables|/Script/Engine.CharacterMovementComponent|SetRotationRate _charactermovement (Math|Rotator|MakeRotator 1.0 1.0 (Math|Conversions|ToFloat(Integer) (Variables|/Game/Data_Assets/BP_DataAssets/BP_DataAssets_Octopus.BP_DataAssets_Octopus_C|GetRotation_Speed _dataassets_octopus))))
  (bind _returnvalue (AddComponent|AddGameplayTasksComponent))
  (Variables|Default|SetTaskWait _returnvalue)
  (Variables|Default|SetAIControllerClass "/Script/AIModule.DetourCrowdAIController")
  (bind _asbp_duck_health (Utilities|Casting|CastToBP_DuckHealth (UserInterface|GetWidget (Variables|Default|GetHealthBar))))
  (Variables|Default|SetHealthBar%20Slider (Variables|/Game/Developers/alexandrecoppens/Collections/BP_DuckHealth.BP_DuckHealth_C|GetHealthBar _asbp_duck_health)))

(event Collision|EventActorBeginOverlap
  (params (OtherActor :type Actor%20Object%20Reference)))

(event EventTick
  (params (DeltaSeconds :type Float%20%28single-precision%29))
  ;[1 1 1] Update
  (CallFunction|CheckHealth)
  (CallFunction|Movement)
  (CallFunction|Effects)
  (CallFunction|Buyancy)
  (CallFunction|UpdateHealthBar))

(event Game|Damage|EventAnyDamage
  (params (Damage :type Float%20%28single-precision%29) (DamageType :type Damage%20Type%20Object%20Reference) (InstigatedBy :type Controller%20Object%20Reference) (DamageCauser :type Actor%20Object%20Reference))
  (bind _charactermovement (Variables|Character|GetCharacterMovement))
  ;[0.169 0.0183 0] Attacked
  (Variables|Default|SetHealth (- (Variables|Default|GetHealth) Damage))
  (if (== DamageType "/Game/GPE/Damage_Type/DT_Classic.DT_Classic")
    (Variables|Default|SetCurrent_Effect DamageType)
    (Variables|/Script/Engine.CharacterMovementComponent|SetMaxWalkSpeed _charactermovement (* (Variables|/Script/Engine.CharacterMovementComponent|GetMaxWalkSpeed _charactermovement) 0.5))))

(fn ConstructionScript)