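; Level manager that creates the player HUD, tracks the remaining BP_Bubble actors and shows the game over screen when none are left.
; On BeginPlay it loads or creates the BP_Save slot; continuing a game destroys bubbles missing from the saved IDs and restores the BP_Portal wave number.
; UpdateNbOfBubble waits a tick, then rebuilds the bubble count and in-memory ID list; only a newly created save is written to disk here.
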(event Custom|UpdateNbOfBubble
  (bind _as_bp_save (Variables|Default|GetAs%20BP%20Save))
  (bind _idbubbles (Variables|/Game/Menus/SaveSystem/BP_Save.BP_Save_C|GetidBubbles _as_bp_save))
  (Utilities|FlowControl|DelayUntilNextTick)
  (bind _outactors (Actor|GetAllActorsOfClass "/Game/GPE/BP_Bubble.BP_Bubble_C"))
  (if (Utilities|Array|IsNotEmpty _outactors)
    (Utilities|Array|Clear _idbubbles)
    (for (_array_element _array_index) _outactors
      (bind _asbp_bubble (Utilities|Casting|CastToBP_Bubble _array_element))
      (Utilities|Array|Add _idbubbles (Variables|/Game/GPE/BP_Bubble.BP_Bubble_C|GetID_Name _asbp_bubble)))
    (bind _result (Math|Integer|IncrementInt _array_index)
      (:%20%20
        (Variables|Default|SetnbOfBubble _result)))
    (else
      (bind _returnvalue (UserInterface|CreateWidget "/Game/Jane/Widgets/WBP_GameOverScreen.WBP_GameOverScreen_C" (Game|GetPlayerController 0)))
      (bind _output_get (Variables|Default|SetGameOver _returnvalue))
      (UserInterface|Viewport|AddtoViewport _output_get 0)
      (Variables|Default|SetnbOfBubble 0))))

(event EventBeginPlay
  (bind _gameover (Variables|Default|GetGameOver))
  ;[1 1 1] UI
  (bind _returnvalue (UserInterface|CreateWidget "/Game/Menus/Viewport/BP_PlayerUI.BP_PlayerUI_C" (Game|GetPlayerController 0)))
  (bind _output_get (Variables|Default|SetNewVar _returnvalue))
  (UserInterface|Viewport|AddtoViewport _output_get 0)
  (CallFunction|UpdateNbOfBubble)
  (if (Utilities|IsValid _gameover)
    (Widget|RemovefromParent _gameover))
  ;[1 0.7742 0] Save system
  (bind _returnvalue_2 (SaveGame|DoesSaveGameExist "GameSave"))
  (if _returnvalue_2
    (bind _returnvalue_3 (SaveGame|LoadGamefromSlot "GameSave"))
    (bind _asbp_save (Utilities|Casting|CastToBP_Save _returnvalue_3))
    (bind _output_get_2 (Variables|Default|SetAs%20BP%20Save _asbp_save))
    ;[1 1 1] Continue game
    (if (Variables|/Game/Menus/SaveSystem/BP_Save.BP_Save_C|GetLoadSave _output_get_2)
      (Variables|/Game/Menus/SaveSystem/BP_Save.BP_Save_C|SetLoadSave _output_get_2 false)
      (bind _outactors (Actor|GetAllActorsOfClass "/Game/GPE/BP_Bubble.BP_Bubble_C"))
      (if (Utilities|Array|IsNotEmpty _outactors)
        (for _array_element _outactors
          (bind _asbp_bubble (Utilities|Casting|CastToBP_Bubble _array_element))
          (if (== -1 (Utilities|Array|FindItem (Variables|/Game/Menus/SaveSystem/BP_Save.BP_Save_C|GetidBubbles _output_get_2) (Variables|/Game/GPE/BP_Bubble.BP_Bubble_C|GetID_Name _asbp_bubble)))
            (Actor|DestroyActor _array_element))
          (bind _returnvalue_4 (Actor|GetActorOfClass "/Game/GPE/BP_Portal.BP_Portal_C"))
          (Utilities|FlowControl|DelayUntilNextTick)
          (Variables|/Game/GPE/BP_Portal.BP_Portal_C|SetWave_Nb _returnvalue_4 (Variables|/Game/Menus/SaveSystem/BP_Save.BP_Save_C|GetnbWave _output_get_2))))
      (else
        ;[0 0 0] new game
        (Utilities|Array|Clear (Variables|/Game/Menus/SaveSystem/BP_Save.BP_Save_C|GetidBubbles _output_get_2))
        (bind _outactors_2 (Actor|GetAllActorsOfClass "/Game/GPE/BP_Bubble.BP_Bubble_C"))
        (if (Utilities|Array|IsNotEmpty _outactors_2)
          (for _array_element_2 _outactors_2
            (bind _asbp_bubble_2 (Utilities|Casting|CastToBP_Bubble _array_element_2))
            (Utilities|Array|Add (Variables|/Game/Menus/SaveSystem/BP_Save.BP_Save_C|GetidBubbles _output_get_2) (Variables|/Game/GPE/BP_Bubble.BP_Bubble_C|GetID_Name _asbp_bubble_2))))))
    (else
      (bind _returnvalue_5 (SaveGame|CreateSaveGameObject "/Game/Menus/SaveSystem/BP_Save.BP_Save_C"))
      (SaveGame|SaveGametoSlot _returnvalue_5 "GameSave")
      (Variables|Default|SetAs%20BP%20Save _returnvalue_5))))

(event EventTick
  (params (DeltaSeconds :type Float%20%28single-precision%29)))

(fn ConstructionScript)