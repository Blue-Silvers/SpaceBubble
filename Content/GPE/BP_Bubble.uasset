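; BP_Bubble is a bubble gameplay actor that reports to the level manager when it is killed.
; Its Kill event finds BP_LevelManager via GetActorOfClass, calls UpdateNbOfBubble, then destroys the actor.
; The construction script stores the object's name in IDName.
; BeginPlay, overlap and Tick are empty, and a loop that destroys the root's child components is left unconnected.
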(event Custom|Kill
  (bind _returnvalue (Actor|GetActorOfClass "/Game/GPE/BP_LevelManager.BP_LevelManager_C"))
  (Default|UpdateNbOfBubble _returnvalue)
  (Actor|DestroyActor))

(event EventBeginPlay)

(event Collision|EventActorBeginOverlap
  (params (OtherActor :type Actor%20Object%20Reference)))

(event EventTick
  (params (DeltaSeconds :type Float%20%28single-precision%29)))

(fn ConstructionScript
  (Variables|Default|SetID_Name (Utilities|GetObjectName self)))