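; BP_BubbleEcplosionForce is a short-lived explosion actor that applies a physical impulse and radial damage for a bubble effect.
; On BeginPlay, UpdateFire copies radius and strengths from a data asset into the radial force component and fires its impulse.
; It then deals DT_BubbleEgg radial damage from the component's location using the same radius, and destroys itself after a brief delay.
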(event EventBeginPlay
  (CallFunction|UpdateFire)
  (Game|Damage|ApplyRadialDamage 5e+01 (Transformation|GetWorldLocation (Variables|Default|GetForceComponent)) (Variables|/Game/Data_Assets/BP_DataAssets/BP_BubbleExplosionDataAsset.BP_BubbleExplosionDataAsset_C|GetBaseRadius (Variables|Default|GetdataAsset)) "/Game/GPE/Damage_Type/DT_BubbleEgg.DT_BubbleEgg_C" 0 0 0 false "ECC_Visibility")
  (Utilities|FlowControl|Delay 0.2)
  (Actor|DestroyActor))

(fn ConstructionScript)

(fn UpdateFire
  (bind _forcecomponent (Variables|Default|GetForceComponent))
  (bind _dataasset (Variables|Default|GetdataAsset))
  (Variables|/Script/Engine.RadialForceComponent|SetRadius _forcecomponent (Variables|/Game/Data_Assets/BP_DataAssets/BP_BubbleExplosionDataAsset.BP_BubbleExplosionDataAsset_C|GetBaseRadius _dataasset))
  (Variables|/Script/Engine.RadialForceComponent|SetImpulseStrength _forcecomponent (Variables|/Game/Data_Assets/BP_DataAssets/BP_BubbleExplosionDataAsset.BP_BubbleExplosionDataAsset_C|GetImpulseStrength _dataasset))
  (Variables|/Script/Engine.RadialForceComponent|SetForceStrength _forcecomponent (Variables|/Game/Data_Assets/BP_DataAssets/BP_BubbleExplosionDataAsset.BP_BubbleExplosionDataAsset_C|GetForceStrength _dataasset))
  (Class|RadialForceComponent|FireImpulse _forcecomponent))